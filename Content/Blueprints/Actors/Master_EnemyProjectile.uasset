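; Master enemy projectile actor that damages what it overlaps and then destroys itself.
; On BeginPlay its Sphere ignores the instigator during movement, and the actor destroys itself after a short delay if nothing triggers it first.
; A separate Sphere1 overlap applies BaseDamage credited to the instigator and its controller, briefly draws the damage result as debug text, then destroys the projectile.
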(event `self.ReceiveBeginPlay`
  (`PrimitiveComponent.IgnoreActorWhenMoving` (`self.Sphere`) (`self.GetInstigator`) true)
  (`KismetSystemLibrary.Delay` 3.0)
  (`self.K2_DestroyActor`))

(event `self.Sphere1.OnComponentBeginOverlap`
  (params (OverlappedComponent :type "PrimitiveComponent Object Reference") (OtherActor :type "Actor Object Reference") (OtherComp :type "PrimitiveComponent Object Reference") (OtherBodyIndex :type Integer) (bFromSweep :type Boolean) (SweepResult :type "HitResult Structure (by ref)"))
  (`/Engine/EditorBlueprintResources/StandardMacros.IsValid` OtherActor
    (:`Is Valid`
      (bind _returnvalue (`GameplayStatics.ApplyDamage` OtherActor (`self.Base Damage`) (`self.GetInstigatorController`) (`self.GetInstigator`)))
      (`KismetSystemLibrary.DrawDebugString` (`self.K2_GetActorLocation`) (`KismetStringLibrary.Conv_DoubleToString` _returnvalue) null (struct :`R` 1.0 :`G` 1.0 :`B` 1.0 :`A` 1.0) 0.3))
    (:`Is Not Valid`
      _))
  (`self.K2_DestroyActor`))

(fn `UserConstructionScript`)