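; Enemy zone actor that spawns a group of enemies within a point budget and alerts them when the player enters its box.
; On BeginPlay it loads enemy classes and costs from the AIManager data table, then greedily fills a capped spawn list.
; The best pick never resets, so the costliest affordable type repeats.
; Enemies spawn at random nearby points, receive the zone as safe zone, and get the player as target on overlap.
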(event `self.ReceiveBeginPlay`
  (set `self.Current_VALUE` (`self.Max_VALUE`))
  (`self.F_GetEnemy_Forces`)
  (for _ (range 1 (+ (`self.SPAWN_max`) 1))
    (`self.F_Distribution_Forces`))
  (for _array_element (`self.Spawn_Forces`)
    (`self.F_Spawn` _array_element)))

(event `Trigger_Characters`
  (for _array_element (`self.Characters`)
    (`/Engine/EditorBlueprintResources/StandardMacros.IsValid` _array_element
      (:`Is Valid`
        (message `/Game/Blueprints/Pawns/AI/Interface/Enemy_Spawn_Interface.GetTarget` _array_element (`self.OtherCharacter`))
        (message `/Game/Blueprints/Pawns/AI/Interface/Enemy_Spawn_Interface.GetSafeZone` _array_element self)))))

(event `self.Box.OnComponentBeginOverlap`
  (params (OverlappedComponent :type "PrimitiveComponent Object Reference") (OtherActor :type "Actor Object Reference") (OtherComp :type "PrimitiveComponent Object Reference") (OtherBodyIndex :type Integer) (bFromSweep :type Boolean) (SweepResult :type "HitResult Structure (by ref)"))
  (bind _asplayer_character (cast `/Game/Blueprints/Pawns/Character/PlayerCharacter` OtherActor))
  (set `self.OtherCharacter` _asplayer_character)
  (`self.Trigger_Characters`))

(fn `F_Distribution_Forces`
  (locals (DT_MaxEnemyValue :type Integer :default 0) (DT_CurrentEnemy :type "/Game/Blueprints/Pawns/AI/Master_Enemy_AI Class Reference") (DT_CurrentValue :type Integer) (DT_AddCurrentEnemy :type "/Game/Blueprints/Pawns/AI/Master_Enemy_AI Class Reference") (SubtractValue :type Integer :default 0))
  (for _array_element (`self.EnemyForces`)
    (bind (_value _class) (break `/Game/Blueprints/Pawns/AI/Data/STR_Enemy_List` _array_element))
    (set `local.DT_CurrentValue` _value)
    (set `local.DT_CurrentEnemy` _class)
    (if (> _value (`self.Max_VALUE`))
      ;[1 1 1] RemoveOverValueEnemy
      (`KismetArrayLibrary.Array_RemoveItem` (`self.EnemyForces`) (make `/Game/Blueprints/Pawns/AI/Data/STR_Enemy_List` (`local.DT_CurrentValue`) (`local.DT_CurrentEnemy`)))
      (elif (< (- (`self.Max_VALUE`) (`local.DT_CurrentValue`)) 0)
        _
        (elif (>= (`local.DT_CurrentValue`) (`local.DT_MaxEnemyValue`))
          (set `local.DT_AddCurrentEnemy` (`local.DT_CurrentEnemy`))
          (set `local.DT_MaxEnemyValue` (`local.DT_CurrentValue`))
          (set `local.SubtractValue` (`local.DT_CurrentValue`))))))
  (if (< (`self.Max_VALUE`) (`local.SubtractValue`))
    (return)
    (else
      (set `self.Max_VALUE` (- (`self.Max_VALUE`) (`local.SubtractValue`)))
      ;[1 1 1] AddEnemyToList
      (`KismetArrayLibrary.Array_Add` (`self.Spawn_Forces`) (`local.DT_AddCurrentEnemy`))
      (return))))

(fn `F_GetEnemy_Forces`
  (bind _ai_manager (`self.AI_Manager`))
  (bind _outrownames (`DataTableFunctionLibrary.GetDataTableRowNames` _ai_manager))
  (for _array_element _outrownames
    (bind _returnvalue (`|GetDataTableRow` _ai_manager _array_element)
      (:`then`
        (`KismetArrayLibrary.Array_AddUnique` (`self.EnemyForces`) _returnvalue))))
  (return))

(fn `F_Spawn`
  (params (Enemy :type "Actor Class Reference"))
  (bind _returnvalue (`|SpawnActorFromClass` Enemy (`KismetMathLibrary.MakeTransform` (`KismetMathLibrary.RandomPointInBoundingBox` (`self.K2_GetActorLocation`) (500.0 500.0 10.0))) "AdjustIfPossibleButAlwaysSpawn" "OverrideRootScale" null null))
  (message `/Game/Blueprints/Pawns/AI/Interface/Enemy_Spawn_Interface.GetSafeZone` _returnvalue self)
  (`KismetArrayLibrary.Array_Add` (`self.Characters`) _returnvalue)
  (return))

(fn `UserConstructionScript`)