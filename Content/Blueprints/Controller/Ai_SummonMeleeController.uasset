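; AI controller for a summoned melee enemy that circles the player and takes turns attacking.
; It moves to randomized points around the player, choosing the closest stored one, while a looping timer re-triggers surrounding if the player gets too far.
; On arrival it faces the player on Tick, then after a random delay either attacks or repositions, capped by counting enemies tagged "Attacking".
; Destruction clears the distance timer and frees a player slot.
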(event Custom|Get%20Circle%20Location
  (Variables|Default|SetPlayerCurrentPostion (Transformation|GetActorLocation (Game|GetPlayerCharacter 0)))
  (Variables|Default|SetTheta (+ (Variables|Default|GetTheta) (Math|Random|RandomFloatinRange 15.0 25.0)))
  (Utilities|Array|Add (Variables|Default|GetLocations) (CallFunction|SetLocations)))

(event Custom|StartAttackingPlayer
  (Variables|Default|SetbLookatPlayer? false)
  (bind _returnvalue (CallFunction|CheckState))
  (if _returnvalue
    (CallFunction|SurroundPlayer)
    (else
      (CallFunction|SwitchState (CallFunction|GetState "NewEnumerator1"))
      (Class|EnemyAnimationInterface|IntFunctionAttackingPlayer(Message) (Pawn|GetControlledPawn)))))

(event EventDestroyed
  (bind _timer_checkdistanceplayerpositions (Variables|Default|GetTimer_CheckDistancePlayerPositions))
  ;[1 1 1] ClearAllTimer
  (if (Utilities|Time|IsValidTimerHandle _timer_checkdistanceplayerpositions)
    (Utilities|Time|ClearandInvalidateTimerbyHandle _timer_checkdistanceplayerpositions)
    (Class|PlayerCharacterInterface|RemoveSlot(Message) (Game|GetPlayerCharacter 0))))

(event EventTick
  (params (DeltaSeconds :type Float%20%28single-precision%29))
  (bind _returnvalue (Pawn|GetControlledPawn))
  (if (Variables|Default|GetbLookatPlayer?)
    (Transformation|SetActorRotation _returnvalue (Math|Rotator|MakeRotator 0.0 0.0 (.Yaw (Math|Rotator|BreakRotator (Math|Rotator|FindLookatRotation (Transformation|GetActorLocation _returnvalue) (Transformation|GetActorLocation (Game|GetPlayerCharacter 0)))))))))

(event EventSurroundPlayer
  (params (PreAtta :type Anim%20Montage%20Object%20Reference))
  (bind _returnvalue (Pawn|GetControlledPawn))
  (Variables|Default|SetPre%20Atta PreAtta)
  (Variables|Default|SetbLookatPlayer? false)
  (Utilities|Time|ClearandInvalidateTimerbyHandle (Variables|Default|GetTimer_Rotation))
  (CallFunction|GetCircleLocation)
  (bind _location (CallFunction|GetClosestLocation))
  (AI|AIMoveTo _returnvalue _location 0 1.5e+02 true
    (:then
      (bind _returnvalue_2 (Utilities|Time|SetTimerbyFunctionName 0 "CheckDistancePlayerPositions" 0.2 true))
      (Variables|Default|SetTimer_CheckDistancePlayerPositions _returnvalue_2))
    (:OnSuccess
      (Class|EnemyAnimationInterface|IntFunctionGetPawnRotation(Message) _returnvalue)
      (Utilities|Array|Clear (Variables|Default|GetLocations))
      (Utilities|Time|SetTimerbyEvent (delegate Custom|StartAttackingPlayer) (Math|Random|RandomFloatinRange 0.55 1.0))
      (Variables|Default|SetbLookatPlayer? true))))

(fn ConstructionScript)

(fn SetLocations
  (bind _returnvalue (Game|GetPlayerCharacter 0))
  (bind _max_radius (Variables|Default|GetMax_Radius))
  (bind _min_radius (Variables|Default|GetMin_Radius))
  (bind _returnvalue_2 (Transformation|GetActorLocation _returnvalue))
  (bind _returnvalue_3 (Math|Random|RandomFloatinRange _min_radius _max_radius))
  (bind (_x _y _z) (Math|Vector|BreakVector _returnvalue_2))
  (bind _output_get (Variables|Default|SetNewLocation (Math|Vector|MakeVector (+ _x (|(R*(Cos({A60CAE12-4346-0C1A-3BD9-558C54BC8937}))) _returnvalue_3)) (+ _y (|(R*(Sin({A60CAE12-4346-0C1A-3BD9-558C54BC8937}))) _returnvalue_3)) _z)))
  (return _output_get))

(fn GetClosestLocation
  (LocalVariables|SetCurrentLocation "0, 0, 0")
  (LocalVariables|SetDistance 1e+05)
  (for _array_element (Variables|Default|GetLocations)
    (if (< (Math|Vector|VectorLength (- _array_element (Transformation|GetActorLocation (Pawn|GetControlledPawn)))) (LocalVariables|GetDistance))
      (LocalVariables|SetDistance (Math|Vector|VectorLength (- _array_element (Transformation|GetActorLocation (Pawn|GetControlledPawn)))))
      (LocalVariables|SetCurrentLocation _array_element)))
  (return (LocalVariables|GetCurrentLocation)))

(fn CheckDistancePlayerPositions
  (if (> (Math|Vector|VectorLength (- (Transformation|GetActorLocation (Game|GetPlayerCharacter 0)) (Transformation|GetActorLocation (Pawn|GetControlledPawn)))) (LocalVariables|GetDistance))
    (Utilities|Time|ClearandInvalidateTimerbyHandle (Variables|Default|GetTimer_CheckDistancePlayerPositions))
    (Class|AiInterface|SurroundPlayer(Message) self)
    (return)
    (else
      (return))))

(fn SwitchState
  (params (Tag :type Name%20%28by%20ref%29))
  (Utilities|Array|AddUnique (Variables|/Script/Engine.Actor|GetTags (Pawn|GetControlledPawn)) Tag)
  (return))

(fn GetState
  (params (Index :type AI_State%20Enum :default "NewEnumerator0"))
  (return (Utilities|Select :Index Index :NewEnumerator0 "Idle" :NewEnumerator1 "Attacking" :NewEnumerator2 "Run")))

(fn CheckState
  (bind _outactors (Actor|GetAllActorsOfClasswithTag "/Game/Blueprints/Pawns/AI/Master_Enemy_AI.Master_Enemy_AI_C" "Attacking"))
  (return (>= (Utilities|Array|Length _outactors) (Variables|Default|GetMaxAttacking))))