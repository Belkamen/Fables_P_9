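; AI controller for a summoner enemy that repositions around the player and summons skeletons.
; SurroundPlayer adds a point at a random radius and advancing angle around the player, then moves to the nearest stored point, retrying on failure.
; On arrival it yaws toward the player each tick, and after a short random delay messages the pawn to summon if at most one SummonSkeleton exists, otherwise repositions.
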(event Custom|Get%20Circle%20Location
  (Variables|Default|SetPlayerCurrentPostion (Transformation|GetActorLocation (Game|GetPlayerCharacter 0)))
  (Variables|Default|SetTheta (+ (Variables|Default|GetTheta) (Math|Random|RandomFloatinRange 15.0 25.0)))
  (Utilities|Array|Add (Variables|Default|GetLocations) (CallFunction|SetLocations)))

(event Custom|StartAttackingPlayer
  (Variables|Default|SetbLookatPlayer? false)
  (bind _outactors (Actor|GetAllActorsOfClass "/Game/Blueprints/Pawns/AI/SummonSkeleton.SummonSkeleton_C"))
  (if (<= (Utilities|Array|Length _outactors) 1)
    (Class|EnemyAnimationInterface|IntFunctionSummoning(Message) (Pawn|GetControlledPawn))
    (else
      (CallFunction|SurroundPlayer))))

(event EventTick
  (params (DeltaSeconds :type Float%20%28single-precision%29))
  (bind _returnvalue (Pawn|GetControlledPawn))
  (if (Variables|Default|GetbLookatPlayer?)
    (Transformation|SetActorRotation _returnvalue (Math|Rotator|MakeRotator 0.0 0.0 (.Yaw (Math|Rotator|BreakRotator (Math|Rotator|FindLookatRotation (Transformation|GetActorLocation _returnvalue) (Transformation|GetActorLocation (Game|GetPlayerCharacter 0)))))))))

(event EventSurroundPlayer
  (params (PreAtta :type Anim%20Montage%20Object%20Reference))
  (bind _returnvalue (Pawn|GetControlledPawn))
  (Variables|Default|SetbLookatPlayer? false)
  (Utilities|Time|ClearandInvalidateTimerbyHandle (Variables|Default|GetTimer_Rotation))
  (CallFunction|GetCircleLocation)
  (bind _location (CallFunction|GetClosestLocation))
  (AI|AIMoveTo _returnvalue _location 0 1.5e+02 true
    (:OnSuccess
      (Class|EnemyAnimationInterface|IntFunctionGetPawnRotation(Message) _returnvalue)
      (Utilities|Array|Clear (Variables|Default|GetLocations))
      (bind _returnvalue_2 (Utilities|Time|SetTimerbyEvent (delegate Custom|StartAttackingPlayer) (Math|Random|RandomFloatinRange 1.0 2.0)))
      (Variables|Default|SetSummoningTimer _returnvalue_2)
      (Variables|Default|SetbLookatPlayer? true))
    (:OnFail
      (CallFunction|SurroundPlayer))))

(fn ConstructionScript)

(fn SetLocations
  (bind _returnvalue (Game|GetPlayerCharacter 0))
  (bind _max_radius (Variables|Default|GetMax_Radius))
  (bind _min_radius (Variables|Default|GetMin_Radius))
  (bind _returnvalue_2 (Transformation|GetActorLocation _returnvalue))
  (bind _returnvalue_3 (Math|Random|RandomFloatinRange _min_radius _max_radius))
  (bind (_x _y _z) (Math|Vector|BreakVector _returnvalue_2))
  (bind _output_get (Variables|Default|SetNewLocation (Math|Vector|MakeVector (+ _x (|(R*(Cos({5FC7E022-4492-B4AF-CF05-EEB16F2968DE}))) _returnvalue_3)) (+ _y (|(R*(Sin({5FC7E022-4492-B4AF-CF05-EEB16F2968DE}))) _returnvalue_3)) _z)))
  (return _output_get))

(fn GetClosestLocation
  (LocalVariables|SetCurrentLocation "0, 0, 0")
  (LocalVariables|SetDistance 1e+05)
  (for _array_element (Variables|Default|GetLocations)
    (if (< (Math|Vector|VectorLength (- _array_element (Transformation|GetActorLocation (Pawn|GetControlledPawn)))) (LocalVariables|GetDistance))
      (LocalVariables|SetDistance (Math|Vector|VectorLength (- _array_element (Transformation|GetActorLocation (Pawn|GetControlledPawn)))))
      (LocalVariables|SetCurrentLocation _array_element)))
  (return (LocalVariables|GetCurrentLocation)))