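; RockTownGameState is a game state that serves quest data and triggers objective markers for interactive characters.
; Its IntQS_GetQuests function reads a QuestTable row, using the first row when no name is given, resets QuestRow, and returns the quest's global name, description and quests.
; GetObjective matches an actor against InteractiveCharacters and calls CreateMarkerMessage on its Marker_Objective component.
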(fn `GetObjective`
  (params (InteractiveActor :type "Actor Object Reference"))
  (locals (Objective :type "ActorComponent Object Reference"))
  (bind _objective (`local.Objective`))
  (for _array_element (`self.InteractiveCharacters`)
    (if (== (`local.InteractiveActor`) _array_element)
      (set `local.Objective` (`self.GetComponentByClass` _array_element "/Game/Blueprints/Pawns/Marker_Objective.Marker_Objective_C"))))
  (`/Engine/EditorBlueprintResources/StandardMacros.IsValid` _objective
    (:`Is Valid`
      (message `/Game/Blueprints/Interface/InteractionActor.CreateMarker` _objective)
      (return))))

(fn `GetRowName`
  (params (RowName :type Name) (Array :type "Array of Name"))
  (returns (ReturnValue :type Name))
  (return (select `bool` (not (== RowName "None")) :`false` (`|GetArrayItem` Array) :`true` (`|GetArrayItem` Array (`KismetArrayLibrary.Array_Find` Array RowName)))))

(fn `IntQS_GetQuests`
  (params (TableName :type Name))
  (returns (Q_GlobalName :type Text) (Q_GlobalDescription :type Text) (Quest :type "Array of /Game/Blueprints/Data/Quests/SubQuestStructure Structure"))
  (locals (QuestName :type Name) (RowNames :type "Array of Name"))
  (bind _questtable (`self.QuestTable`))
  (bind _outrownames (`DataTableFunctionLibrary.GetDataTableRowNames` _questtable))
  (set `local.RowNames` _outrownames)
  (set `local.QuestName` (`self.GetRowName` TableName (`local.RowNames`)))
  (bind _returnvalue (`|GetDataTableRow` _questtable (`local.QuestName`))
    (:`then`
      (set `self.QuestRow` 0)
      (bind (_global_name _global_description _quests) (break `/Game/Blueprints/Data/Quests/GlobalQuest_Structure` _returnvalue))
      (return _global_name _global_description _quests))))

(fn `UserConstructionScript`)