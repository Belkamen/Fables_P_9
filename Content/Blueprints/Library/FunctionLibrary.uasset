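; Blueprint function library of shared helpers for the top-down controller, dialogue UI and quest state.
; It fetches player 0's TopDownController, creates dialogue and answer widgets on the viewport, and reads or writes GlobalQuests on the GameInstance.
; Theta uses sine and cosine math expressions to place a point on a horizontal circle around an actor.
; SaveGame is a stub that only checks whether a slot exists.
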(fn SaveGame
  (params (SlotName :type String))
  (bind _returnvalue (SaveGame|DoesSaveGameExist SlotName))
  (if _returnvalue
    _))

(fn GetController
  (bind _astop_down_controller (Utilities|Casting|CastToTopDownController (Game|GetPlayerController 0)))
  (return _astop_down_controller))

(fn CreateDialogue
  (params (OwningPlayer :type Player%20Controller%20Object%20Reference))
  (bind _returnvalue (UserInterface|CreateWidget "/Game/Blueprints/Widgets/Dialogue/Dialogue_Widget.Dialogue_Widget_C" OwningPlayer))
  (UserInterface|Viewport|AddtoViewport _returnvalue 0)
  (return _returnvalue))

(fn CreateAnswer
  (params (OwningPlayer :type Player%20Controller%20Object%20Reference))
  (bind _returnvalue (UserInterface|CreateWidget "/Game/Blueprints/Widgets/Dialogue/Answer_Widget.Answer_Widget_C" OwningPlayer))
  (UserInterface|Viewport|AddtoViewport _returnvalue 0)
  (return _returnvalue))

(fn Theta
  (params (Angle :type Float%20%28double-precision%29) (Origin :type Actor%20Object%20Reference))
  (bind _returnvalue (Transformation|GetActorLocation Origin))
  (bind _radius (LocalVariables|GetRadius))
  (bind (_x _y _z) (Math|Vector|BreakVector _returnvalue))
  (LocalVariables|SetTheta Angle)
  (return (Math|Vector|MakeVector (+ _x (|(R*(Cos({B880D39E-4621-D9B0-2BAA-C4A2B60CBB4A}))) _radius)) (+ _y (|(R*(Sin({B880D39E-4621-D9B0-2BAA-C4A2B60CBB4A}))) _radius)) _z)))

(fn GlobalQuestID
  (bind _asgame_instance (Utilities|Casting|CastToGameInstance (Game|GetGameInstance (LocalVariables|Get__WorldContext))))
  (return (Variables|/Game/Blueprints/Main/GameInstance.GameInstance_C|GetGlobalQuests _asgame_instance)))

(fn SetGlobalQuestID
  (params (GlobalQuests :type Integer))
  (bind _asgame_instance (Utilities|Casting|CastToGameInstance (Game|GetGameInstance (LocalVariables|Get__WorldContext))))
  (Variables|/Game/Blueprints/Main/GameInstance.GameInstance_C|SetGlobalQuests _asgame_instance GlobalQuests)
  (return))